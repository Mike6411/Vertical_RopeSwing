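; Grapple hook component that fires a hook projectile with an attached cable and pulls the owning character toward where it hits.
; A state enum drives it: firing spawns and binds hook and cable, and a hit launches the owner with gravity and friction off.
; Tick keeps pulling until wallrunning, proximity, or passing the hook horizontally (2D dot product) destroys the hook.
; The hook's destroyed event centralizes cleanup, removing the cable and resetting state and movement values.
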(event `self.ReceiveTick`
  (params (DeltaSeconds :type "Float (single-precision)"))
  (switch `/Game/Blueprints/GrappleHook/EGrappleHook` (`self.GrappleState`)
    (:`NewEnumerator2`
      (bind _ascharacter (cast `Character` (`self.GetOwner`)))
      (`CharacterMovementComponent.AddForce` (`Character.CharacterMovement` _ascharacter) (* (`self.ToGrappleHook`) (`self.GrapplePullforce`)))
      ;[1 1 1] Prevencion de que se este usando elgrapple y wallruning a la vez
      (bind _asbp_player_char (cast `/Game/Blueprints/BP_PlayerChar` (`self.GetOwner`)))
      (if (`/Game/Blueprints/BP_PlayerChar.IsWallrunning?` _asbp_player_char)
        (`Actor.K2_DestroyActor` (`self.GrappleHook`))
        (else
          ;[1 1 1] Si estamos lo suficientemente cerca del Grapple destruye el Grapple
          (if (< (`KismetMathLibrary.Vector_Distance` (`Actor.K2_GetActorLocation` (`self.GrappleHook`)) (`Actor.K2_GetActorLocation` (`self.GetOwner`))) (`self.DistanceToGrappleCutoff`))
            (`Actor.K2_DestroyActor` (`self.GrappleHook`))
            (elif (< (`KismetMathLibrary.Dot_VectorVector` (`self.InitialHookDirection2D`) (`self.ToGrappleHook2D`)) 0.0)
              (`Actor.K2_DestroyActor` (`self.GrappleHook`)))))))))

(fn `CancelGrapple`
  ;[1 1 1] Setup para hacer el cleanup en On Grapple Hook Destroyed
  (bind _grapplehook (`self.GrappleHook`)
    (:`then`
      (`Actor.K2_DestroyActor` _grapplehook))
    (:`else`)))

(fn `FireGrapple`
  (params (TargetLocation :type "Vector Structure") (LocalOffset :type "Vector Structure"))
  (locals (FireDirection :type "Vector Structure" :default (0.0 0.0 0.0)))
  (if (not (`self.IsInUse?`))
    (set `self.GrappleState` "NewEnumerator1")
    (set `local.FireDirection` (`KismetMathLibrary.Normal` (- (`local.TargetLocation`) (`self.CableStartLocation` (`local.LocalOffset`)))))
    (bind _returnvalue (`|SpawnActorFromClass` "/Game/Blueprints/GrappleHook/BP_Grapple_Hook.BP_Grapple_Hook_C" (`KismetMathLibrary.MakeTransform` (`self.CableStartLocation` (`local.LocalOffset`))) "Undefined" "MultiplyWithRoot" null (* (`local.FireDirection`) (`self.GrappleSpeed`)) null))
    ;[1 1 1] Bindeamos los eventos de collision y destrucción aqui en el component
    (bind _output_get (set `self.GrappleHook` _returnvalue))
    (add `Actor.OnActorHit` _output_get (`|CreateDelegate` :!event `OnGrappleHit`))
    (add `Actor.OnDestroyed` (`self.GrappleHook`) (`|CreateDelegate` :!event `OnGrappleHookDestroyed`))
    (bind _returnvalue_2 (`|SpawnActorFromClass` "/Game/Blueprints/GrappleHook/CP_GrappleCable.CP_GrappleCable_C" (`KismetMathLibrary.MakeTransform` (`self.CableStartLocation` (`local.LocalOffset`)) (`KismetMathLibrary.MakeRotFromX` (`local.FireDirection`))) "Undefined" "MultiplyWithRoot" null null))
    ;[1 1 1] Enganchamos las dos puntas del cable. El principio al punto de disparo del jugador y el final al grapple en si
    (bind _output_get_2 (set `self.GrappleCable` _returnvalue_2))
    ;;[1 1 1] Usamos Keep World ya que aun que attachamos el cable al jugador no queremos cambiar donde esta el cable
    (`Actor.K2_AttachToActor` _output_get_2 (`self.GetOwner`) "None" "KeepWorld" "KeepWorld" "KeepWorld" true)
    (`CableComponent.SetAttachEndTo` (`CableActor.CableComponent` (`self.GrappleCable`)) (`self.GrappleHook`) "None" "None")
    ;;[1 1 1] Le quitamos el offset que lleva por defecto el cable
    (set `CableComponent.EndLocation` (0.0 0.0 0.0) (`CableActor.CableComponent` (`self.GrappleCable`)))))

(fn `IsInUse?`
  (returns (Result :type Boolean))
  (return (select `/Game/Blueprints/GrappleHook/EGrappleHook` (`self.GrappleState`) :`NewEnumerator1` true :`NewEnumerator2` true)))

(fn `OnGrappleHit`
  (params (SelfActor :type "Actor Object Reference") (OtherActor :type "Actor Object Reference") (NormalImpulse :type "Vector Structure") (Hit :type "HitResult Structure (by ref)"))
  (set `self.GrappleState` "NewEnumerator2")
  (bind _ascharacter (cast `Character` (`self.GetOwner`)))
  (bind _charactermovement (`Character.CharacterMovement` _ascharacter))
  (set `CharacterMovementComponent.GroundFriction` 0.0 _charactermovement)
  (set `CharacterMovementComponent.GravityScale` 0.0 _charactermovement)
  (set `CharacterMovementComponent.AirControl` 0.4 _charactermovement)
  (set `MovementComponent.Velocity` (* (`self.ToGrappleHook`) (`self.GrapplePullforceInitial`)) _charactermovement)
  (set `self.InitialHookDirection2D` (`self.ToGrappleHook2D`)))

(fn `OnGrappleHookDestroyed`
  (params (DestroyedActor :type "Actor Object Reference"))
  ;[1 1 1] Cleanup de los diferentes componentes del grapple y reset del GrappleState
  (set `self.GrappleHook` null)
  (set `self.GrappleState` "NewEnumerator0")
  (`|ExecutionSequence`
    (:`then_0`
      (bind _grapplecable (`self.GrappleCable`)
        (:`then`
          (`Actor.K2_DestroyActor` _grapplecable)
          (set `self.GrappleCable` null))
        (:`else`)))
    (:`then_1`
      ;[1 1 1] Volver los valores a sus defaults
      (bind _ascharacter (cast `Character` (`self.GetOwner`)))
      (bind _charactermovement (`Character.CharacterMovement` _ascharacter))
      (set `CharacterMovementComponent.GroundFriction` 1.0 _charactermovement)
      (set `CharacterMovementComponent.GravityScale` 1.0 _charactermovement)
      (set `CharacterMovementComponent.AirControl` 0.05 _charactermovement))))