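; BP_FinishLine is a trigger actor that starts and stops the player's timer when the player crosses it.
; On BeginPlay it caches player 0's character as BP_PlayerChar.
; When that character begins overlapping the Box, a FlipFlop alternates the character's PauseTimer flag, so the first crossing unpauses the timer and the next pauses it.
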(event `self.ReceiveBeginPlay`
  (bind _asbp_player_char (cast `/Game/Blueprints/BP_PlayerChar` (`GameplayStatics.GetPlayerCharacter` 0)))
  (set `self.As BP Player Char` _asbp_player_char))

(event `self.Box.OnComponentBeginOverlap`
  (params (OverlappedComponent :type "PrimitiveComponent Object Reference") (OtherActor :type "Actor Object Reference") (OtherComp :type "PrimitiveComponent Object Reference") (OtherBodyIndex :type Integer) (bFromSweep :type Boolean) (SweepResult :type "HitResult Structure (by ref)"))
  (bind _as_bp_player_char (`self.As BP Player Char`))
  (if (== OtherActor (`self.As BP Player Char`))
    (`/Engine/EditorBlueprintResources/StandardMacros.FlipFlop`
      (:`A`
        (set `/Game/Blueprints/BP_PlayerChar.PauseTimer` false _as_bp_player_char))
      (:`B`
        (set `/Game/Blueprints/BP_PlayerChar.PauseTimer` true _as_bp_player_char)))))

(fn `UserConstructionScript`)