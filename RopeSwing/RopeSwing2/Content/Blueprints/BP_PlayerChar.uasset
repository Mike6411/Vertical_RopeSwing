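; Player character with wallrunning, multi-jump, sprint, a grapple hook, two switchable cameras and a level-restart input.
; BeginPlay adds the Enhanced Input context and HUD and timer widgets; a camera trace targets GrappleComponent.
; Capsule hits while falling start wallruns, where timelines re-trace the wall, steer velocity and roll the view, with gravity off.
; Jumps use LaunchCharacter, pushing away from walls; the Tick-called horizontal speed clamp is disconnected.
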(event `self.ReceiveBeginPlay`
  (bind _returnvalue (pcsubsystem `EnhancedInputLocalPlayerSubsystem` (`GameplayStatics.GetPlayerController` 0)))
  ;[1 1 1] INP y Widget setup
  (`self.Reset Jump` (`self.MaxJumps`))
  (`MovementComponent.SetPlaneConstraintEnabled` (`self.CharacterMovement`) true)
  (`/Engine/EditorBlueprintResources/StandardMacros.IsValid` _returnvalue
    (:`Is Valid`
      (`EnhancedInputSubsystemInterface.AddMappingContext` _returnvalue "/Game/Inputs/IMC_ThirdP.IMC_ThirdP" 0 (struct))
      (bind _returnvalue_2 (`|CreateWidget` "/Game/Widgets/W_MainHUD.W_MainHUD_C"))
      (`UserWidget.AddToViewport` _returnvalue_2 0)
      (bind _returnvalue_3 (`|CreateWidget` "/Game/Widgets/W_Timer.W_Timer_C"))
      (`UserWidget.AddToViewport` _returnvalue_3 0))))

(event `EnhancedInput|/Game/Inputs/INP_FireGrapple`
  (params (ActionValue :type Boolean) (ElapsedSeconds :type "Float (double-precision)") (TriggeredSeconds :type "Float (double-precision)") (InputAction :type "InputAction Object Reference" :default "/Game/Inputs/INP_FireGrapple.INP_FireGrapple"))
  (bind _grapplecomponent (`self.GrappleComponent`))
  (bind _camera (`self.Camera`))
  (bind _returnvalue (`SceneComponent.K2_GetComponentLocation` _camera))
  ;[0 1 0.1775] Grapple Hook
  (:`Started`
    (if (`/Game/Blueprints/GrappleHook/GrappleComponent.IsInUse?` _grapplecomponent)
      (`/Game/Blueprints/GrappleHook/GrappleComponent.CancelGrapple` _grapplecomponent)
      (else
        (bind (_outhit _returnvalue_2) (`KismetSystemLibrary.LineTraceSingle` _returnvalue (+ _returnvalue (* (`SceneComponent.GetForwardVector` _camera) 10000.0)) "TraceTypeQuery1"))
        (bind (_bblockinghit _binitialoverlap _time _distance _location _impactpoint _normal _impactnormal _physmat _hitactor _hitcomponent _hitbonename _bonename _hititem _elementindex _faceindex _tracestart _traceend) (`GameplayStatics.BreakHitResult` _outhit))
        (`/Game/Blueprints/GrappleHook/GrappleComponent.FireGrapple` (`self.GrappleComponent`) (select `bool` _returnvalue_2 :`false` _traceend :`true` _location) (30.0 0.0 60.0))))))

(event `EnhancedInput|/Game/Inputs/INP_Look`
  (params (ActionValue :type "Vector2D Structure") (ElapsedSeconds :type "Float (double-precision)") (TriggeredSeconds :type "Float (double-precision)") (InputAction :type "InputAction Object Reference" :default "/Game/Inputs/INP_Look.INP_Look"))
  ;[1 1 1] Movimiento Base
  (:`Triggered`
    (`self.AddControllerYawInput` ActionValue_X)
    (`self.AddControllerPitchInput` ActionValue_Y)))

(event `self.OnLanded`
  (params (Hit :type "HitResult Structure (by ref)"))
  ;[0 0.01813 1] Wallrun
  (`self.Reset Jump` (`self.MaxJumps`)))

(event `EnhancedInput|/Game/Inputs/INP_Jump`
  (params (ActionValue :type Boolean) (ElapsedSeconds :type "Float (double-precision)") (TriggeredSeconds :type "Float (double-precision)") (InputAction :type "InputAction Object Reference" :default "/Game/Inputs/INP_Jump.INP_Jump"))
  ;[0 0.01813 1] Wallrun
  (:`Started`
    (`self.ConsumeJump`
      (:`Consumed`
        ;;[1 1 1] El salto en si
        (`self.LaunchCharacter` (`self.FindLaunchVel`) false true)
        (`self.OnWall`
          (:`true`
            ;;[1 1 1] La unica version de end reason que termina con JumpOffWall
            (`self.EndWallrun` "NewEnumerator1"))))))
  (:`Completed`
    (`self.StopJumping`)))

(event `EnhancedInput|/Game/Inputs/INP_Move`
  (params (ActionValue :type "Vector2D Structure") (ElapsedSeconds :type "Float (double-precision)") (TriggeredSeconds :type "Float (double-precision)") (InputAction :type "InputAction Object Reference" :default "/Game/Inputs/INP_Move.INP_Move"))
  (bind (_returnvalue_roll _returnvalue_pitch _returnvalue_yaw) (`KismetMathLibrary.BreakRotator` (`self.GetControlRotation`)))
  ;[1 1 1] Movimiento Base
  (:`Triggered`
    (set `self.ForwardAxis` ActionValue_Y)
    (set `self.RightAxis` ActionValue_X)
    (`self.AddMovementInput` (`KismetMathLibrary.GetRightVector` (`self.GetControlRotation`)) ActionValue_X)
    (`self.AddMovementInput` (`KismetMathLibrary.GetForwardVector` (`KismetMathLibrary.MakeRotator` _returnvalue_roll 0.0 _returnvalue_yaw)) ActionValue_Y)))

(event `EnhancedInput|/Game/Inputs/INP_Sprint`
  (params (ActionValue :type Boolean) (ElapsedSeconds :type "Float (double-precision)") (TriggeredSeconds :type "Float (double-precision)") (InputAction :type "InputAction Object Reference" :default "/Game/Inputs/INP_Sprint.INP_Sprint"))
  ;[1 1 1] Movimiento Base
  (:`Triggered`
    (`self.Sprint`))
  (:`Completed`
    (`self.Stop sprint`)))

(event `Reset Jump`
  (params (Jumps :type Integer))
  ;[0 0.01813 1] Wallrun
  (set `self.JumpsLeft` (`KismetMathLibrary.Clamp` Jumps 0 (`self.MaxJumps`))))

(event `EnhancedInput|/Game/Inputs/INP_Camswitch`
  (params (ActionValue :type Boolean) (ElapsedSeconds :type "Float (double-precision)") (TriggeredSeconds :type "Float (double-precision)") (InputAction :type "InputAction Object Reference" :default "/Game/Inputs/INP_Camswitch.INP_Camswitch"))
  (bind _camera (`self.Camera`))
  (bind _camera2 (`self.Camera2`))
  ;[1 0.1936 0] Camera Switch
  (:`Started`
    (if (`ActorComponent.IsActive` (`self.Camera`))
      (`ActorComponent.SetActive` _camera2 true false)
      (`ActorComponent.SetActive` _camera false false)
      (else
        (`ActorComponent.SetActive` _camera2 false false)
        (`ActorComponent.SetActive` _camera true false)))))

(event `EnhancedInput|/Game/Inputs/INP_ResetMap`
  (params (ActionValue :type Boolean) (ElapsedSeconds :type "Float (double-precision)") (TriggeredSeconds :type "Float (double-precision)") (InputAction :type "InputAction Object Reference" :default "/Game/Inputs/INP_ResetMap.INP_ResetMap"))
  (:`Started`
    (`/Engine/EditorBlueprintResources/StandardMacros.DoOnce` false
      (:`Completed`
        (`KismetSystemLibrary.ExecuteConsoleCommand` "RestartLevel" null)))))

(event `self.CapsuleComponent.OnComponentHit`
  (params (HitComponent :type "PrimitiveComponent Object Reference") (OtherActor :type "Actor Object Reference") (OtherComp :type "PrimitiveComponent Object Reference") (NormalImpulse :type "Vector Structure") (Hit :type "HitResult Structure (by ref)"))
  (bind (_direction _side) (`self.FindRunDirectionAndSide` Hit_ImpactNormal))
  ;[0 0.01813 1] Wallrun
  (`self.OnWall`
    (:`false`
      (if (`self.CanSurfaceBeWallran` Hit_ImpactNormal)
        (if (`NavMovementComponent.IsFalling` (`self.CharacterMovement`))
          (set `self.WallrunDir` _direction)
          (set `self.WallrunSide` _side)
          (if (`self.AreRequiredKeysDown`)
            (`self.BeginWallrun`)))))))

(event `self.ReceiveTick`
  (params (DeltaSeconds :type "Float (single-precision)"))
  ;[0 0.01813 1] Wallrun
  (`self.ClampHorizontalVel`))

(event `BeginWallrun`
  (bind _charactermovement (`self.CharacterMovement`))
  ;[0 0.01813 1] Wallrun
  (set `CharacterMovementComponent.AirControl` 1.0 _charactermovement)
  (set `CharacterMovementComponent.GravityScale` 0.0 _charactermovement)
  (`MovementComponent.SetPlaneConstraintNormal` _charactermovement (0.0 0.0 1.0))
  (set `self.IsWallrunning?` true)
  (`self.BeginCameraTilt`)
  (`Timeline|UpdateWallrunTimeline` :!label _label
    (:`Update`
      (`self.UpdateWallrun`))))

(event `EndWallrun`
  (params (EndReason :type "/Game/Blueprints/Wallrun/EWallrunEndReason Enum" :default "NewEnumerator0"))
  (bind _charactermovement (`self.CharacterMovement`))
  ;[0 0.01813 1] Wallrun
  ;;[1 1 1] Si te caes de la pared tienes un salto si no no te quedan
  (`self.Reset Jump` (select `/Game/Blueprints/Wallrun/EWallrunEndReason` EndReason :`NewEnumerator0` 1 :`NewEnumerator1` (- (`self.MaxJumps`) 1)))
  (set `CharacterMovementComponent.AirControl` 0.05 _charactermovement)
  (set `CharacterMovementComponent.GravityScale` 1.0 _charactermovement)
  (`MovementComponent.SetPlaneConstraintNormal` _charactermovement (0.0 0.0 0.0))
  (`self.EndCameraTilt`)
  (set `self.IsWallrunning?` false)
  (goto _label :!via `Stop`))

(event `BeginCameraTilt`
  (bind _returnvalue (`self.GetController`))
  (bind (_returnvalue_roll _returnvalue_pitch _returnvalue_yaw) (`KismetMathLibrary.BreakRotator` (`Controller.GetControlRotation` _returnvalue)))
  ;[0 0.01813 1] Wallrun
  (bind (_direction _roll) (`Timeline|UpdateTickTimeline` :!label _label_2)
    (:`Update`
      (`Controller.SetControlRotation` _returnvalue (`KismetMathLibrary.MakeRotator` (* _roll (select `/Game/Blueprints/Wallrun/EWallrunSide` (`self.WallrunSide`) :`NewEnumerator0` -1.0 :`NewEnumerator1` 1.0 :!type "Float (single-precision)")) _returnvalue_pitch _returnvalue_yaw)))))

(event `EndCameraTilt`
  ;[0 0.01813 1] Wallrun
  (goto _label_2 :!via `Reverse`))

(fn `AreRequiredKeysDown`
  (returns (Return :type Boolean))
  (if (> (`self.ForwardAxis`) 0.1)
    (switch `/Game/Blueprints/Wallrun/EWallrunSide` (`self.WallrunSide`)
      (:`NewEnumerator0`
        (return (> (`self.ForwardAxis`) 0.1)))
      (:`NewEnumerator1`
        (return (> (`self.ForwardAxis`) 0.1))))
    (else
      (return false))))

(fn `CanSurfaceBeWallran`
  (params (`Surface Normal` :type "Vector Structure"))
  (returns (NewParam :type Boolean))
  (bind (_x _y _z) (`KismetMathLibrary.BreakVector3f` `Surface Normal`))
  ;[1 1 1] Miramos que no sea el techo o angulada hacia nosotros
  (if (< _z -0.05)
    (return false)
    (else
      (return (< (`KismetMathLibrary.DegAcos` (`KismetMathLibrary.Dot_VectorVector` (`KismetMathLibrary.Normal` (`KismetMathLibrary.MakeVector` _x _y)) `Surface Normal`)) (`CharacterMovementComponent.K2_GetWalkableFloorAngle` (`self.CharacterMovement`)))))))

(fn `ClampHorizontalVel`
  ;[1 1 1] Esto existe porque al usar el Launch Character para el salto en el segundo salto te da un impulso en la direccion en la que te mueves (aparte del vertical) y esto lo convierte de nuevo un salto normal. Esto tiene que estar desactivado cuando el Grapple se esta usando obviamente. Sry por usarlo en el event tick pero al ser algo que al llamarse devuelve el negativo muy frequentemente pues no creo que sea lo peor :p
)

(fn `FindLaunchVel`
  (returns (`Launch Velocity` :type "Vector Structure"))
  (locals (LaunchDir :type "Vector Structure"))
  (bind _camera (`self.Camera`))
  (`|ExecutionSequence`
    (:`then_0`
      (if (`self.IsWallrunning?`)
        (set `local.LaunchDir` (`KismetMathLibrary.Cross_VectorVector` (`self.WallrunDir`) (select `/Game/Blueprints/Wallrun/EWallrunSide` (`self.WallrunSide`) :`NewEnumerator0` (0.0 0.0 1.0) :`NewEnumerator1` (0.0 0.0 -1.0) :!type "Vector Structure")))
        (elif (`NavMovementComponent.IsFalling` (`self.CharacterMovement`))
          (set `local.LaunchDir` (+ (* (`self.RightAxis`) (`SceneComponent.GetRightVector` _camera)) (* (`self.ForwardAxis`) (`SceneComponent.GetForwardVector` _camera)))))))
    (:`then_1`
      (return (* (+ (`local.LaunchDir`) (0.0 0.0 1.0)) (`CharacterMovementComponent.JumpZVelocity` (`self.CharacterMovement`)))))))

(fn `FindRunDirectionAndSide`
  (params (`Wall Normal` :type "Vector Structure"))
  (returns (Direction :type "Vector Structure") (Side :type "/Game/Blueprints/Wallrun/EWallrunSide Enum"))
  (locals (SideLocal :type "/Game/Blueprints/Wallrun/EWallrunSide Enum"))
  (bind _output_get (set `local.SideLocal` (select `bool` (> (`KismetMathLibrary.DotProduct2D` (`KismetMathLibrary.Conv_VectorToVector2D` `Wall Normal`) (`KismetMathLibrary.Conv_VectorToVector2D` (`self.GetActorRightVector`))) 0.0) :`false` "NewEnumerator0" :`true` "NewEnumerator1" :!type "/Game/Blueprints/Wallrun/EWallrunSide Enum")))
  (return (`KismetMathLibrary.Cross_VectorVector` (`local.Wall Normal`) (select `/Game/Blueprints/Wallrun/EWallrunSide` _output_get :`NewEnumerator0` (0.0 0.0 -1.0) :`NewEnumerator1` (0.0 0.0 1.0) :!type "Vector Structure")) (`local.SideLocal`)))

(fn `GetHorizontalVel`
  (returns (ReturnValue :type "Vector2D Structure"))
  (return (`KismetMathLibrary.Conv_VectorToVector2D` (`MovementComponent.Velocity` (`self.CharacterMovement`)))))

(fn `SetHorizontalVel`
  (params (`Horizontal Vel` :type "Vector2D Structure"))
  (bind _charactermovement (`self.CharacterMovement`))
  (bind (_velocity_x _velocity_y _velocity_z) (`KismetMathLibrary.BreakVector` (`MovementComponent.Velocity` _charactermovement)))
  (set `MovementComponent.Velocity` (`KismetMathLibrary.MakeVector` `Horizontal Vel_X` `Horizontal Vel_Y` _velocity_z) _charactermovement))

(fn `Sprint`
  (set `CharacterMovementComponent.MaxWalkSpeed` (`self.Sprintspeed`) (`self.CharacterMovement`)))

(fn `Stop sprint`
  (set `CharacterMovementComponent.MaxWalkSpeed` (`self.Walkspeed`) (`self.CharacterMovement`)))

(fn `UpdateWallrun`
  (bind _returnvalue (`self.K2_GetActorLocation`))
  (bind _charactermovement (`self.CharacterMovement`))
  ;[1 1 1] Mirar si estamos aguantando las teclas correctas, si no es que te has caido
  (if (`self.AreRequiredKeysDown`)
    ;[1 1 1] Linetrace para ver i hay una pared
    (bind (_outhit _returnvalue_2) (`KismetSystemLibrary.LineTraceSingle` _returnvalue (+ _returnvalue (* (`KismetMathLibrary.Cross_VectorVector` (`self.WallrunDir`) (select `/Game/Blueprints/Wallrun/EWallrunSide` (`self.WallrunSide`) :`NewEnumerator0` (0.0 0.0 -1.0) :`NewEnumerator1` (0.0 0.0 1.0) :!type "Vector Structure")) 200.0)) "TraceTypeQuery1"))
    (if _returnvalue_2
      (bind (_direction _side) (`self.FindRunDirectionAndSide` (`.ImpactNormal` (`GameplayStatics.BreakHitResult` _outhit))))
      (if (`|EnumEquality` _side (`self.WallrunSide`))
        ;[1 1 1] Si no ha cambiado queremos updatear la velocidad basandonos en nuestra wallrun dir
        (bind _output_get (set `self.WallrunDir` _direction))
        (bind (_returnvalue_x _returnvalue_y) (`KismetMathLibrary.BreakVector` (* _output_get (`MovementComponent.GetMaxSpeed` _charactermovement))))
        (set `MovementComponent.Velocity` (`KismetMathLibrary.MakeVector` _returnvalue_x _returnvalue_y) _charactermovement)
        (else
          (`self.EndWallrun` "NewEnumerator0")))
      (else
        ;[1 1 1] Te has quedado sin pared
        (`self.EndWallrun` "NewEnumerator0")))
    (else
      (`self.EndWallrun` "NewEnumerator0"))))

(fn `UserConstructionScript`)